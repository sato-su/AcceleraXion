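; AI controller for team-based enemy bots: runs BT_Enemy, assigns red or blue team with its default rifle, and spawns that weapon on respawn.
; Perception feeds the Blackboard: sight and damage share an opposing-team tag check, but only sight writes target, focus and last known location.
; Hearing sets a heard flag and redirects the patrol point to the sound.
; Timers delay reactions to lost sight and heard sounds.
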(event OnTargetPerceptionUpdated(AIPerception)
  (params (Actor :type Actor%20Object%20Reference) (Stimulus :type AI%20Stimulus%20Structure))
  ;[1 1 1] 敵発見時
  (Variables|Default|SetSensedActor Actor)
  (bind _returnvalue (Class|AIPerceptionSystem|GetSenseClassforStimulus Stimulus))
  (switch string (Utilities|GetClassDisplayName _returnvalue)
    (:AISense_Sight
      (CallFunction|HandleSightSense Stimulus :!label _label))
    (:AISense_Damage
      (goto _label))
    (:AISense_Hearing
      (CallFunction|HandleHearingSense Stimulus))))

(event Custom|SetRandomLocation
  (params (VectorValue :type Vector))
  (AI|Components|Blackboard|SetValueasVector (Variables|Default|GetBlackboard) (Utilities|Name|MakeLiteralName "RandomLocation") VectorValue))

(event Custom|SelectWeaponAIC
  (params (SelectedWeapon :type BP%20Weapon%20Base%20Class%20Reference))
  ;[1 1 1] リスポーン時の初期装備
  (Variables|Default|SetSelectedWeapon SelectedWeapon))

(event Custom|RespawnWeaponsAIC
  (params (SpawnTransform :type Transform) (PlayerBase :type BP%20Player%20Base%20Object%20Reference))
  ;[1 1 1] リスポーン時の初期装備
  (bind _returnvalue (Game|SpawnActorfromClass (Variables|Default|GetSelectedWeapon) SpawnTransform "Undefined" "MultiplyWithRoot" 0 0))
  (bind _output_get (Variables|Default|SetRifle _returnvalue))
  (Default|SRVSetInitialWeapons PlayerBase _output_get))

(event Custom|SetTeam
  (params (Condition :type Boolean))
  (if Condition
    (Variables|Default|SetTeam "/Game/Blueprints/AI/BP_BlueAI.BP_BlueAI_C")
    (Variables|Default|SetSelectedWeapon "/Game/Blueprints/Weapons/BP_M4A1.BP_M4A1_C")
    (else
      (Variables|Default|SetTeam "/Game/Blueprints/AI/BP_RedAI.BP_RedAI_C")
      (Variables|Default|SetSelectedWeapon "/Game/Blueprints/Weapons/BP_AK47.BP_AK47_C"))))

(event Custom|LoseTaget
  ;[1 1 1] 敵発見時
  (AI|Components|Blackboard|SetValueasObject (Variables|Default|GetBlackboard) (Utilities|Name|MakeLiteralName "TargetActor") 0) ; 見失ったら削除
  (AI|ClearFocus))

(event Custom|FalseCanHearPlayer
  ;[1 1 1] 敵発見時
  (AI|Components|Blackboard|SetValueasBool (Variables|Default|GetBlackboard) (Utilities|Name|MakeLiteralName "CanHearPlayer") false))

(event EventBeginPlay
  (AI|RunBehaviorTree "/Game/Blueprints/AI/BT_Enemy.BT_Enemy"))

(fn ConstructionScript)

(fn WriteActorLocation
  (params (Actor :type Actor%20Object%20Reference) (Stimulus :type AI%20Stimulus%20Structure))
  (bind _returnvalue (Class|AIPerceptionSystem|GetSenseClassforStimulus Stimulus))
  (if (== _returnvalue "/Script/AIModule.AISense_Sight")
    (AI|Components|Blackboard|SetValueasObject (Variables|Default|GetBlackboard) (Utilities|Name|MakeLiteralName "TargetActor") Actor)
    (AI|SetFocus Actor)
    (AI|Components|Blackboard|SetValueasVector (Variables|Default|GetBlackboard) (Utilities|Name|MakeLiteralName "LastKnownLocation") (.stimuluslocation Stimulus))
    (else
      (return))))

(fn HandleSightSense
  (params (AIStimulus :type AI%20Stimulus%20Structure))
  (bind _sensedactor (Variables|Default|GetSensedActor))
  ;[1 1 1] チームが違うプレイヤー見つけた場合
  (if (== (Variables|Default|GetTeam) "/Game/Blueprints/AI/BP_BlueAI.BP_BlueAI_C")
    (if (Actor|ActorHasTag _sensedactor "RedSide")
      (if (Utilities|Struct|BreakAIStimulus AIStimulus) :!label _label
        (CallFunction|WriteActorLocation (Variables|Default|GetSensedActor) AIStimulus) ; 見えたら、アクタとその位置をブラックボードに書き込む
        (Utilities|Time|ClearandInvalidateTimerbyHandle (Variables|Default|GetLoseTargetTimer))
        (bind _asbp_ai (Utilities|Casting|CastToBP_AI (Pawn|GetControlledPawn)))
        (AI|Components|Blackboard|SetValueasFloat (Variables|Default|GetBlackboard) (Utilities|Name|MakeLiteralName "AIHealth") (Variables|/Game/Blueprints/Player/BP_PlayerBase.BP_PlayerBase_C|GetCurrentHealth _asbp_ai))
        (else
          (bind _returnvalue (Utilities|Time|SetTimerbyEvent (EventDispatchers|CreateEvent :!event Custom|LoseTaget) 3.0))
          (Variables|Default|SetLoseTargetTimer _returnvalue))))
    (elif (Actor|ActorHasTag _sensedactor "BlueSide")
      (goto _label))))

(fn HandleHearingSense
  (params (AIStimulus :type AI%20Stimulus%20Structure))
  (bind (_age _expirationage _strength _stimuluslocation _receiverlocation _tag _bsuccessfullysensed) (Utilities|Struct|BreakAIStimulus AIStimulus))
  (AI|Components|Blackboard|SetValueasBool (Variables|Default|GetBlackboard) (Utilities|Name|MakeLiteralName "CanHearPlayer") _bsuccessfullysensed)
  (if _bsuccessfullysensed
    (AI|Components|Blackboard|SetValueasVector (Variables|Default|GetBlackboard) (Utilities|Name|MakeLiteralName "PatrolPoint") _stimuluslocation)
    (bind _returnvalue (Utilities|Time|SetTimerbyEvent (EventDispatchers|CreateEvent :!event Custom|FalseCanHearPlayer) 5.0))
    (Variables|Default|SetHearTimer _returnvalue)))

(fn GetAIControllerRef
  (return self))