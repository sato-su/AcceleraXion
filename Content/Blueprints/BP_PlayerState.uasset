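; BP_PlayerState is a player state Blueprint that tracks a player's kill count, death count and team.
; Setter events write the Kill, Death and Team variables, each of which has a RepNotify function.
; Those functions call the matching OnKillChanged, OnDeathChanged and OnTeamChanged dispatchers, so listeners can react to replicated changes.
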(event Custom|SetPlayerKill
  (params (Kill :type Integer))
  (Variables|Default|SetKill Kill))

(event Custom|SetPlayerDeath
  (params (Death :type Integer))
  (Variables|Default|SetDeath Death))

(event Custom|SetPlayerTeam
  (params (Team :type E_Team%20Enum :default "NewEnumerator0"))
  (Variables|Default|SetTeam Team))

(fn ConstructionScript)

(fn OnRepKill
  (Default|CallOnKillChanged))

(fn OnRepDeath
  (Default|CallOnDeathChanged))

(fn OnRepTeam
  (Default|CallOnTeamChanged))