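; Base weapon actor that simulates physics and can be looted by players.
; On BeginPlay a server event fills ammo and fire timing from weapon info looked up by name.
; Server-side sphere overlaps offer it to players lacking that weapon type, skipping whoever just dropped it, and clear the dropped-weapon reference on exit.
; Lifespan events schedule or cancel destruction, with a shorter timer for empty weapons.
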(event OnComponentBeginOverlap(CollisionSphere)
  (params (OverlappedComponent :type Primitive%20Component%20Object%20Reference) (OtherActor :type Actor%20Object%20Reference) (OtherComp :type Primitive%20Component%20Object%20Reference) (OtherBodyIndex :type Integer) (bFromSweep :type Boolean) (SweepResult :type Hit%20Result%20Structure%20%28by%20ref%29))
  (bind _overlappingactors (Collision|GetOverlappingActors "/Game/Blueprints/Player/BP_PlayerBase.BP_PlayerBase_C" :!class /Script/Engine.Actor))
  (if (Actor|ActorHasTag OtherActor "Character") ; Playerタグが付いたActorが範囲内ならTrue
    (Networking|SwitchHasAuthority ; サーバー介して実行
      (:Authority
        (if (Variables|Default|GetbCanBeInteractedWith)
          (if (> (Utilities|Array|Length _overlappingactors) 1)
            (bind _array_element (Utilities|Array|ForEachLoopwithBreak _overlappingactors :!label _label)
              (:LoopBody
                (bind _player (Class|INTPlayerBase|GetPlayerRef(Message) _array_element))
                (if (!= (Variables|/Game/Blueprints/Player/BP_PlayerBase.BP_PlayerBase_C|GetDroppedWeapon _player) self)
                  (Variables|Default|SetInteractiongPlayer _player)
                  (goto _label Break)))
              (:Completed
                (bind _array_element_2 (Utilities|Array|ForEachLoopwithBreak (Variables|/Game/Blueprints/Player/BP_PlayerBase.BP_PlayerBase_C|GetWeaponInventory (stale _interactiongplayer)) :!label _label_2)
                  (:LoopBody
                    (if (Utilities|Enum|Equal(Enum) (.Type (Utilities|Struct|BreakST_WeaponInfo (CallFunction|FGetWeaponInfo (Variables|BP_WeaponBase_C|GetWeaponName _array_element_2)))) (.Type (Utilities|Struct|BreakST_WeaponInfo (CallFunction|FGetWeaponInfo (Variables|Default|GetWeaponName)))))
                      (Variables|/Game/Blueprints/Player/BP_PlayerBase.BP_PlayerBase_C|SetbCanLootWeapon (Variables|Default|GetInteractiongPlayer) false)
                      (goto _label_2 Break)))
                  (:Completed
                    (if (Variables|/Game/Blueprints/Player/BP_PlayerBase.BP_PlayerBase_C|GetbCanLootWeapon (Variables|Default|GetInteractiongPlayer))
                      (Default|AddOverlappedWeapon (Variables|Default|GetInteractiongPlayer) self)
                      (else
                        (Variables|/Game/Blueprints/Player/BP_PlayerBase.BP_PlayerBase_C|SetbCanLootWeapon (Variables|Default|GetInteractiongPlayer) true)))))))
            (else
              (bind _player_2 (Class|INTPlayerBase|GetPlayerRef(Message) (Utilities|Array|Get(acopy) _overlappingactors)))
              (Utilities|IsValid _player_2
                (:Is%20Valid
                  (if (!= (Variables|/Game/Blueprints/Player/BP_PlayerBase.BP_PlayerBase_C|GetDroppedWeapon _player_2) self)
                    (Variables|Default|SetInteractiongPlayer _player_2)
                    (bind _interactiongplayer (Variables|Default|GetInteractiongPlayer)
                      (:then
                        (goto _label_2))
                      (:else)))))))
          (else
            (Utilities|FlowControl|Delay 0.1)))))))

(event OnComponentEndOverlap(CollisionSphere)
  (params (OverlappedComponent :type Primitive%20Component%20Object%20Reference) (OtherActor :type Actor%20Object%20Reference) (OtherComp :type Primitive%20Component%20Object%20Reference) (OtherBodyIndex :type Integer))
  (if (Actor|ActorHasTag OtherActor "Character") ; Characterタグが付いたActorが範囲内ならTrue
    (Networking|SwitchHasAuthority
      (:Authority
        (bind _player (Class|INTPlayerBase|GetPlayerRef(Message) OtherActor))
        (Default|SetDroppedWeapon _player)))))

(event Custom|SRV_InitializeWeapon
  (bind _weaponname (Variables|Default|GetWeaponName))
  (bind _weaponinfo (CallFunction|FGetWeaponInfo _weaponname))
  (bind (_maxammoinmag _maxextraammo _headdamage _chestdamage _bodydamage _otherpartsdamage _firingrate) (Utilities|Struct|BreakST_WeaponInfo _weaponinfo))
  (Variables|Default|SetCurrentAmmoInMag _maxammoinmag)
  (Variables|Default|SetCurrentExtraAmmo _maxextraammo)
  (bind _output_get (Variables|Default|SetFiringRate _firingrate))
  (Variables|Default|SetFiringCoolTime (/ 6e+01 _output_get)))

(event Custom|DestroyingWeapon
  (if (and (== (Variables|Default|GetCurrentExtraAmmo) 0) (== (Variables|Default|GetCurrentAmmoInMag) 0))
    (Actor|SetLifeSpan 5.0)
    (else
      (Actor|SetLifeSpan 2e+01))))

(event Custom|DestroyWeapon
  (Actor|DestroyActor))

(event Custom|StopDestroy
  (Actor|SetLifeSpan 0.0))

(event EventBeginPlay
  (Physics|SetSimulatePhysics (Variables|Default|GetWeapon) true)
  (CallFunction|SRVInitializeWeapon))

(fn ConstructionScript)

(fn GetWeaponRef
  (return self))