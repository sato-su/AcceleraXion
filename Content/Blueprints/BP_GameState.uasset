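; Game State Blueprint for a Red vs Blue team match, holding the round timer, both team scores, the max score and the player state list.
; Simple events set or increment these values and add or remove unique player states.
; RepNotify functions broadcast timer, score and player list changes through event dispatchers, while MaxScore's notify is empty and only rides along with score broadcasts.
; KillDeath relays killer and victim states directly through its own dispatcher.
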(event Custom|SetRoundTimer
  (params (RoundTimer :type Float%20%28double-precision%29))
  (Variables|Default|SetRoundTimer RoundTimer))

(event Custom|SetMaxScore
  (params (MaxScore :type Integer))
  (Variables|Default|SetMaxScore MaxScore))

(event Custom|PlusScoreBlue
  (Variables|Default|SetScoreBlue (+ (Variables|Default|GetScoreBlue) 1)))

(event Custom|SetScoreBlue
  (params (ScoreBlue :type Integer))
  (Variables|Default|SetScoreBlue ScoreBlue))

(event Custom|SetScoreRed
  (params (ScoreRed :type Integer))
  (Variables|Default|SetScoreRed ScoreRed))

(event Custom|PlusScoreRed
  (Variables|Default|SetScoreRed (+ (Variables|Default|GetScoreRed) 1)))

(event Custom|SetPlayerStates
  (params (NewPlayerState :type BP%20Player%20State%20Object%20Reference))
  (Utilities|Array|AddUnique (Variables|Default|GetPlayerStates) NewPlayerState))

(event Custom|DeletePlayerStates
  (params (PlayerState :type BP%20Player%20State%20Object%20Reference))
  (Utilities|Array|RemoveItem (Variables|Default|GetPlayerStates) PlayerState))

(event Custom|KillDeath
  (params (killerState :type BP%20Player%20State%20Object%20Reference) (DeadState :type BP%20Player%20State%20Object%20Reference))
  (Default|CallOnKillDeath killerState DeadState))

(fn ConstructionScript)

(fn OnRepRoundTimer
  (Default|CallOnTimeChanged (Variables|Default|GetRoundTimer)))

(fn OnRepScoreBlue
  (Default|CallOnBlueScoreChanged (Variables|Default|GetScoreBlue) (Variables|Default|GetMaxScore)))

(fn OnRepScoreRed
  (Default|CallOnRedScoreChanged (Variables|Default|GetScoreRed) (Variables|Default|GetMaxScore)))

(fn OnRepMaxScore)

(fn OnRepPlayerStates
  (Default|CallOnPlayerStateChanged))