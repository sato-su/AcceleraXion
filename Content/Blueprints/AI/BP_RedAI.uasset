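; BP_RedAI is an AI character Blueprint that places itself on a team, apparently Red, when play begins.
; After the parent BeginPlay, it sets the team flag to false on its AIC_AcceleraXion controller, then assigns the matching team enum on its BP_PlayerState.
; The two casts run in sequence, so a failed controller cast also skips the player state update.
; Construction only calls the parent, and Tick and overlap events are empty.
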(event EventBeginPlay
  (|CallParentFunction)
  (bind _asaic_accelera_xion (Utilities|Casting|CastToAIC_AcceleraXion (Variables|Default|GetAIC_AcceleraXion)))
  (Default|SetTeam _asaic_accelera_xion false)
  (bind _asbp_player_state (Utilities|Casting|CastToBP_PlayerState (Variables|Default|GetPlayerState)))
  (Default|SetPlayerTeam _asbp_player_state "NewEnumerator1"))

(event Collision|EventActorBeginOverlap
  (params (OtherActor :type Actor%20Object%20Reference)))

(event EventTick
  (params (DeltaSeconds :type Float%20%28single-precision%29)))

(fn ConstructionScript
  (|CallParentFunction))