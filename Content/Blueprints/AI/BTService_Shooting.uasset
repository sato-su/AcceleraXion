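; A behavior tree service that makes an AI-controlled BP_AI pawn shoot at its focus actor when it has a clear line of sight.
; On activation it caches the controlled pawn as BP_AI.
; Each tick it sphere-traces on the Camera channel from the pawn to the controller's focus actor, ignoring itself, and calls FireBullet only if the first hit is that actor.
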(event EventReceiveActivationAI
  (params (OwnerController :type AI%20Controller%20Object%20Reference) (ControlledPawn :type Pawn%20Object%20Reference))
  (bind _asbp_ai (Utilities|Casting|CastToBP_AI ControlledPawn))
  (Variables|Default|SetAs%20BP%20AI _asbp_ai)
  (Variables|Default|SetOwner%20Controller OwnerController))

(event EventReceiveTickAI
  (params (OwnerController :type AI%20Controller%20Object%20Reference) (ControlledPawn :type Pawn%20Object%20Reference) (DeltaSeconds :type Float%20%28single-precision%29))
  (bind (_outhit _returnvalue) (Collision|SphereTraceByChannel (Transformation|GetActorLocation ControlledPawn) (Transformation|GetActorLocation (Class|AIController|GetFocusActor OwnerController)) 0.0 "TraceTypeQuery2" false (Utilities|Array|MakeArray (Variables|Default|GetAs%20BP%20AI)) "None"))
  (if _returnvalue
    (if (== (.HitActor (Collision|BreakHitResult _outhit)) (Class|AIController|GetFocusActor (Variables|Default|GetOwner%20Controller)))
      (Default|FireBullet (Variables|Default|GetAs%20BP%20AI)))))