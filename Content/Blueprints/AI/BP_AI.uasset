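; AI-controlled shooter character that fires at the actor its AI controller is focused on.
; On possession it caches the AI controller for use by the FireBullet event.
; FireBullet aims from the S_Camera socket slightly above the focus actor's location, randomizes direction within a cone, then calls AIshoot and AIStopShoot.
; An invisible debug visibility trace precedes the shot; its result is unused and its random direction is computed separately.
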(event Custom|FireBullet
  (bind _mesh (Variables|Character|GetMesh))
  (bind _aic_acceleraxion (Variables|Default|GetAIC_AcceleraXion))
  (bind _returnvalue (Class|AIController|GetFocusActor _aic_acceleraxion))
  (bind _returnvalue_2 (Transformation|GetSocketLocation _mesh "S_Camera"))
  (bind _returnvalue_3 (Transformation|GetActorLocation _returnvalue))
  (bind (_x _y _z) (Math|Vector|BreakVector _returnvalue_3))
  (bind _returnvalue_4 (+ _z 3e+01))
  (bind _returnvalue_5 (Math|Vector|MakeVector _x _y _returnvalue_4))
  (bind _returnvalue_6 (- _returnvalue_5 _returnvalue_2))
  (bind _returnvalue_7 (Math|Vector|Normalize _returnvalue_6))
  (bind _returnvalue_8 (Math|Random|RandomUnitVectorinConeinDegrees _returnvalue_7 1e+01))
  (bind _returnvalue_9 (* _returnvalue_8 1e+04))
  (bind _returnvalue_10 (+ _returnvalue_2 _returnvalue_9))
  (Utilities|IsValid _returnvalue
    (:Is%20Valid
      (Collision|MultiLineTraceByChannel _returnvalue_2 _returnvalue_10 "TraceTypeQuery1" false 0 "None") ; Debug
      (CallFunction|AIshoot _returnvalue_2 _returnvalue_10)
      (CallFunction|AIStopShoot))))

(event EventBeginPlay
  (|CallParentFunction))

(event EventPossessed
  (params (NewController :type Controller%20Object%20Reference))
  (bind _asaicontroller (Utilities|Casting|CastToAIController NewController))
  (Utilities|IsValid _asaicontroller
    (:Is%20Valid
      (Variables|Default|SetAIC_AcceleraXion _asaicontroller))))

(fn ConstructionScript
  (|CallParentFunction))