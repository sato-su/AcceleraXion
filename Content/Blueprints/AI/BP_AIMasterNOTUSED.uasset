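; Master AI enemy Blueprint, marked unused by its name, that roams the NavMesh and chases players it sees.
; A delayed event loop picks random reachable points, while PawnSensing sightings set InRange and redirect movement to the player.
; Tick checks speed, running and jumping to control a looping timer that plays footsteps through server and multicast events.
; A hearing-based move is left disconnected, and comments plan footsteps for a Behavior Tree.
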(event OnSeePawn(PawnSensing)
  (params (Pawn :type Pawn%20Object%20Reference))
  ;[1 1 1 1 50] プレイヤー発見時
  (Variables|Default|SetInRange true)
  (bind _asbp_player_base (Utilities|Casting|CastToBP_PlayerBase Pawn))
  (AI|AIMoveTo self "0, 0, 0" _asbp_player_base 5e+01 false
    (:then
      (CallFunction|DecideNextAction))))

(event Custom|DecideNextAction
  ;[1 1 1 1 50] 次アクション
  (Utilities|FlowControl|Delay 0.5)
  (CallFunction|RandomRoam))

(event Custom|RandomRoam
  ;[1 1 1 1 50] ランダム移動
  (if (Variables|Default|GetInRange)
    (Variables|Default|SetInRange false)
    (else
      (Variables|/Script/Engine.CharacterMovementComponent|SetMaxWalkSpeed (Variables|Character|GetCharacterMovement) 9e+02)
      (AI|AIMoveTo self (.RandomLocation (AI|Navigation|GetRandomReachablePointinRadius (Transformation|GetActorLocation) 1e+03 0 0)) 0 5.0 false
        (:OnSuccess
          (Development|PrintString "randooooo"))
        (:OnFail
          (Development|PrintString "Failed RAndom")))
      (CallFunction|DecideNextAction))))

(event Custom|CustomEvent
  ;[1 0.01342 0 1 50] 足音 Behavior Treeで実装予定
  (CallFunction|SRVPlayFootstepsSFX))

(event Custom|CustomEvent_1
  ;[1 0.01342 0 1 50] 足音 Behavior Treeで実装予定
  (CallFunction|MCPlayFootstepsSFX))

(event Custom|CustomEvent_2
  ;[1 0.01342 0 1 50] 足音 Behavior Treeで実装予定
  (Audio|PlaySoundatLocation "/Game/Audio/SFX/SC_Footsteps.SC_Footsteps" (Transformation|GetActorLocation) "0, 0, 0" 1.0 1.0 0.0 0 0 0 0))

(event EventBeginPlay
  (|CallParentFunction)
  (CallFunction|RandomRoam))

(event EventTick
  (params (DeltaSeconds :type Float%20%28single-precision%29))
  ;[1 0.01342 0 1 50] 足音 Behavior Treeで実装予定
  (if (Math|Boolean|ANDBoolean (>= (Math|Vector|VectorLengthSquared (Transformation|GetVelocity)) 9.1e+04) (CallFunction|FIsRunning) (CallFunction|FIsNotJumping)) ; false分岐で走りからの姿勢変更でも足音消える
    (if (not (Variables|Default|GetPlayingFootstepsSFX))
      (Variables|Default|SetPlayingFootstepsSFX true)
      (CallFunction|SRVPlayFootstepsSFX) ; 最初の足音
      (bind _returnvalue (Utilities|Time|SetTimerbyEvent (delegate Custom|CustomEvent) 0.4 true))
      (Variables|Default|SetFootstepsSFXTimerHandle _returnvalue))
    (elif (Utilities|Time|IsValidTimerHandle (Variables|Default|GetFootstepsSFXTimerHandle))
      (Utilities|Time|ClearandInvalidateTimerbyHandle (Variables|Default|GetFootstepsSFXTimerHandle)) ; 足音タイマー停止
      (Variables|Default|SetPlayingFootstepsSFX false))))

(fn ConstructionScript
  (|CallParentFunction))