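; Multiplayer base player character with Enhanced Input movement, look, crouch, walk, jump and weapon pickup, hiding its head bone on setup.
; Crouch, walk and aim pitch replay through server RPCs; the last MovementState entry sets speed.
; A looping timer multicasts running footsteps through the server.
; The server loots queued overlapped weapons, and OnRep_LootedWeapon disables their physics and collision, attaching them to hand or holster sockets.
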(event Custom|SRV_Crouch
  (params (bCrouch :type Boolean))
  ;[1 1 1] しゃがみ
  (CallFunction|FCrouch bCrouch))

(event Custom|SRV_Walk
  (params (bWalk :type Boolean))
  ;[1 1 1] 歩き
  (CallFunction|FWalk bWalk))

(event Custom|AddOverlappedWeapon
  (params (Weapon :type BP%20Weapon%20Base%20Object%20Reference))
  ;[1 1 1] 武器取得
  (CallFunction|SRVAddOverlappedWeapon Weapon))

(event Custom|SRV_AddOverlappedWeapon
  (params (Weapon :type BP%20Weapon%20Base%20Object%20Reference))
  (bind _overlappedweapons (Variables|Default|GetOverlappedWeapons))
  ;[1 1 1] 武器取得
  (Utilities|Array|SetArrayElem _overlappedweapons (Utilities|Array|Length _overlappedweapons) Weapon true) ; Size to Fitにチェックつけないと取得できなくなる
  (Utilities|FlowControl|DoOnce false
    (:Completed
      (CallFunction|LootWeapon))))

(event Custom|CheckForOverlappedWeapon
  ;[1 1 1] 武器取得
  (CallFunction|LootWeapon))

(event Custom|CanLootWeaponAgain
  ;[1 1 1] 武器取得
  (Utilities|FlowControl|DoOnce false) ; enters at Reset
)

(event Custom|SRV_CalculateAimDirection
  ;[1 1 1] 視点中心計算(アニメーション用)
  (CallFunction|FCalculateAimDirection))

(event Custom|PlayFootstepsSFX
  ;[1 1 1] 足音
  (CallFunction|SRVPlayFootstepsSFX))

(event Custom|SRV_PlayFootstepsSFX
  ;[1 1 1] 足音
  (CallFunction|MCPlayFootstepsSFX))

(event Custom|MC_PlayFootstepsSFX
  ;[1 1 1] 足音
  (Audio|PlaySoundatLocation "/Game/Audio/SFX/SC_Footsteps.SC_Footsteps" (Transformation|GetActorLocation) "0, 0, 0" 1.0 1.0 0.0 0 0 0 0))

(event Custom|LootWeapon
  ;[1 1 1] 武器取得
  (CallFunction|SRVLootWeapon))

(event Custom|SRV_LootWeapon
  (bind _weaponinventory (Variables|Default|GetWeaponInventory))
  (bind _overlappedweapons (Variables|Default|GetOverlappedWeapons))
  (bind _output (Utilities|Array|Get(acopy) _overlappedweapons))
  ;[1 1 1] 武器取得
  (if (Utilities|Array|IsNotEmpty _overlappedweapons)
    (Utilities|Array|SetArrayElem _weaponinventory (Utilities|Array|Length _weaponinventory) _output true)
    (Variables|Default|SetLootedWeapon _output) ; OnRep_LootedWeaponが実行
    (if (Utilities|Enum|Equal(Enum) (Variables|Default|GetEquippedWeapon) "NewEnumerator0")
      (Utilities|FlowControl|Delay 0.2) ; rip完了待機用
      (CallFunction|SetEquippedWeapon (Variables|/Game/Blueprints/Weapons/BP_WeaponBase.BP_WeaponBase_C|GetWeaponType (Variables|Default|GetLootedWeapon)))
      (Utilities|Array|RemoveItem (Variables|Default|GetOverlappedWeapons) _output)
      (CallFunction|CheckforOverlappedWeapon) ; ループさせる事で重なった武器を同時に取得可能
    )
    (else
      (CallFunction|CanLootWeaponAgain))))

(event Custom|SetEquippedWeapon
  (params (EquippedWeapon :type E_WeaponType%20Enum :default "NewEnumerator0"))
  ;[1 1 1] 武器取得
  (CallFunction|SRVSetEquippedWeapon EquippedWeapon))

(event Custom|SRV_SetEquippedWeapon
  (params (EquippedWeapon :type E_WeaponType%20Enum :default "NewEnumerator0"))
  ;[1 1 1] 武器取得
  (Variables|Default|SetEquippedWeapon EquippedWeapon))

(event Input|EnhancedActionEvents|EnhancedInputActionIA_Movement
  (params (ActionValue :type Vector%202D%20Structure) (ElapsedSeconds :type Float%20%28double-precision%29) (TriggeredSeconds :type Float%20%28double-precision%29) (InputAction :type Input%20Action%20Object%20Reference :default "/Game/Blueprints/Player/Input/IA_Movement.IA_Movement"))
  ;[1 1 1] WASD移動
  (:Triggered
    (Pawn|Input|AddMovementInput (Transformation|GetActorForwardVector) (.x ActionValue) false) ; 前後の移動\nwでScaleValue1\nSで-1
    (Pawn|Input|AddMovementInput (Transformation|GetActorRightVector) (.y ActionValue) false) ; 左右の移動
    ;[1 1 1] 足音
    (if (Math|Boolean|ANDBoolean (>= (Math|Vector|VectorLengthSquared (Transformation|GetVelocity)) 9.1e+04) (CallFunction|FIsRunning) (CallFunction|FIsNotJumping) (> TriggeredSeconds 0.2)) ; false分岐で走りからの姿勢変更でも足音消える
      (if (not (Variables|Default|GetPlayingFootstepsSFX))
        (Variables|Default|SetPlayingFootstepsSFX true)
        (CallFunction|SRVPlayFootstepsSFX) ; 最初の足音
        (bind _returnvalue (Utilities|Time|SetTimerbyEvent (delegate Custom|PlayFootstepsSFX) 0.4 true))
        (Variables|Default|SetFootstepsSFXTimerHandle _returnvalue))
      (else
        (if (Utilities|Time|IsValidTimerHandle (Variables|Default|GetFootstepsSFXTimerHandle)) :!label _label
          (Utilities|Time|ClearandInvalidateTimerbyHandle (Variables|Default|GetFootstepsSFXTimerHandle)) ; 足音タイマー停止
          (Variables|Default|SetPlayingFootstepsSFX false)))))
  (:Completed
    (goto _label)))

(event Input|EnhancedActionEvents|EnhancedInputActionIA_Look
  (params (ActionValue :type Vector%202D%20Structure) (ElapsedSeconds :type Float%20%28double-precision%29) (TriggeredSeconds :type Float%20%28double-precision%29) (InputAction :type Input%20Action%20Object%20Reference :default "/Game/Blueprints/Player/Input/IA_Look.IA_Look"))
  ;[1 1 1] 視点移動
  (:Triggered
    (Pawn|Input|AddControllerYawInput (.x ActionValue)) ; 左右視点移動
    (Pawn|Input|AddControllerPitchInput (.y ActionValue)) ; 上下視点移動\n入力マップでyだけnegateにすると\nマウス前で上空見る
    ;[1 1 1] 視点中心計算(アニメーション用)
    (CallFunction|FCalculateAimDirection)))

(event Input|EnhancedActionEvents|EnhancedInputActionIA_Crouch
  (params (ActionValue :type Boolean) (ElapsedSeconds :type Float%20%28double-precision%29) (TriggeredSeconds :type Float%20%28double-precision%29) (InputAction :type Input%20Action%20Object%20Reference :default "/Game/Blueprints/Player/Input/IA_Crouch.IA_Crouch"))
  ;[1 1 1] しゃがみ
  (:Triggered
    (if (CallFunction|FIsNotJumping) :!label _label ; ジャンプ中のしゃがみ防止
      (if ActionValue ; アクションマッピングでPressedとReleasedをトリガーに追加したので、\n押した時True、話した時Falseが実行
        (CallFunction|FCrouch true)
        (elif (Utilities|Array|ContainsItem (Variables|Default|GetMovementState) "NewEnumerator2") ; ジャンプ中しゃがみ入力を\n離していたらUncrouchしない
          (CallFunction|FCrouch false)))
      (else
        (Utilities|FlowControl|Delay 0.05) ; ジャンプ中にしゃがみ入力\nしていたら着地時しゃがむ
        (goto _label)))))

(event Input|EnhancedActionEvents|EnhancedInputActionIA_Walk
  (params (ActionValue :type Boolean) (ElapsedSeconds :type Float%20%28double-precision%29) (TriggeredSeconds :type Float%20%28double-precision%29) (InputAction :type Input%20Action%20Object%20Reference :default "/Game/Blueprints/Player/Input/IA_Walk.IA_Walk"))
  ;[1 1 1] 歩き
  (:Triggered
    (if ActionValue
      (CallFunction|FWalk true)
      (else
        (CallFunction|FWalk false)))))

(event Input|EnhancedActionEvents|EnhancedInputActionIA_Jump
  (params (ActionValue :type Boolean) (ElapsedSeconds :type Float%20%28double-precision%29) (TriggeredSeconds :type Float%20%28double-precision%29) (InputAction :type Input%20Action%20Object%20Reference :default "/Game/Blueprints/Player/Input/IA_Jump.IA_Jump"))
  ;[1 1 1] ジャンプ
  (:Triggered
    (if (CallFunction|FIsNotJumping) ; 飛行中・液体中・地上ならジャンプできる
      (Character|Jump) ; これだけでサーバー・クライアント実装可能
    )))

(event EventBeginPlay
  ;[1 1 1] 実行時
  (Utilities|FlowControl|Delay 0.01) ; 接続待機用遅延
  (bind _playercontroller (Class|INTPlayerController|GetPlayerControllerRef(Message) (Pawn|GetController))) ; メッセージアイコンはBPインターフェースから来た事を示す。\nCastToは参照取得(ハード参照)。BP通信はBPインターフェースのが良い。\nハード参照について：\nhttps://okawari-hakumai.hatenablog.com/entry/2020/10/30/194341
  (Utilities|IsValid _playercontroller
    (:Is%20Valid
      (Utilities|IsValid (PlayerController|LocalPlayerSubsystems|GetEnhancedInputLocalPlayerSubsystem _playercontroller)
        (:Is%20Valid
          (Input|AddMappingContext (PlayerController|LocalPlayerSubsystems|GetEnhancedInputLocalPlayerSubsystem _playercontroller) "/Game/Blueprints/Player/Input/IMC_Default.IMC_Default" 0 "(bIgnoreAllPressedKeysUntilRelease=True,bForceImmediately=False)") ; 使用マッピングを追加
          (Components|SkinnedMesh|HideBonebyName (Variables|Character|GetMesh) "head" "PBO_None"))))))

(fn ConstructionScript)

(fn FCrouch
  (params (bCrouch :type Boolean))
  (bind _movementstate (Variables|Default|GetMovementState))
  (bind _output_get (LocalVariables|SetCrouchLocal bCrouch))
  (Networking|SwitchHasAuthority ; Authはサーバー側\nRemoteはクライアント側
    (:Authority
      _)
    (:Remote
      (CallFunction|SRVCrouch _output_get) ; サーバーがしゃがみ実行後、クライアント側がしゃがめる
    ))
  (if (LocalVariables|GetCrouchLocal) ; Authからのみつなぐとサーバー側のプレイヤーのみしゃがめる
    (Character|Crouch)
    (Utilities|Array|SetArrayElem _movementstate (+ (Utilities|Array|LastIndex _movementstate) 1) "NewEnumerator2" true) ; しゃがんでいるかどうかを列挙で管理。\nADDだとマルチプレイヤーでバグ多い為、こちらを用いる
    (CallFunction|FSetMovementSpeed)
    (else
      (Character|UnCrouch)
      (Utilities|Array|RemoveItem (Variables|Default|GetMovementState) "NewEnumerator2")
      (CallFunction|FSetMovementSpeed))))

(fn FWalk
  (params (bWalk :type Boolean))
  (bind _movementstate (Variables|Default|GetMovementState))
  (bind _output_get (LocalVariables|SetWalk%20Local bWalk))
  (Networking|SwitchHasAuthority ; Authはサーバー側\nRemoteはクライアント側
    (:Authority
      _)
    (:Remote
      (CallFunction|SRVWalk _output_get)))
  (if (LocalVariables|GetWalk%20Local)
    (Utilities|Array|SetArrayElem _movementstate (+ (Utilities|Array|LastIndex _movementstate) 1) "NewEnumerator1" true) ; ADDだとマルチプレイヤーでバグ多い為、こちらを用いる
    (CallFunction|FSetMovementSpeed)
    (else
      (Utilities|Array|RemoveItem (Variables|Default|GetMovementState) "NewEnumerator1")
      (CallFunction|FSetMovementSpeed))))

(fn FIsNotJumping
  (return (not (AI|Components|NavMovement|IsFalling (Variables|Character|GetCharacterMovement)))))

(fn FSetMovementSpeed
  (bind _movementstate (Variables|Default|GetMovementState))
  (bind _movementstate_2 (Variables|Default|GetMovementState))
  (if (Utilities|Enum|Equal(Enum) (Utilities|Array|Get(acopy) _movementstate (Utilities|Array|LastIndex _movementstate)) "NewEnumerator2") ; この処理により、しゃがみ→歩き同時押しの際に、しゃがみ速度で歩きモーションになるバグを修正
    (Character|Crouch)
    (else
      (Character|UnCrouch)))
  (Variables|/Script/Engine.CharacterMovementComponent|SetMaxWalkSpeed (Variables|Character|GetCharacterMovement) (Utilities|Select :Index (Utilities|Array|Get(acopy) _movementstate_2 (Utilities|Array|LastIndex _movementstate_2)) :NewEnumerator0 (Variables|Default|GetRunSpeed) :NewEnumerator1 (Variables|Default|GetWalkSpeed) :NewEnumerator2 (Variables|Default|GetCrouchSpeed))))

(fn FCalculateAimDirection
  (Networking|SwitchHasAuthority
    (:Authority
      _)
    (:Remote
      (CallFunction|SRVCalculateAimDirection)))
  (Variables|Default|SetAimDirection (.Pitch (Math|Rotator|BreakRotator (Math|Rotator|Delta(Rotator) (Pawn|GetControlRotation :!class /Script/Engine.Pawn) (Transformation|GetActorRotation))))) ; サーバーのみ実行。\nクライアント側はサーバーを介してのみ実行。
)

(fn FIsRunning
  (bind _movementstate (Variables|Default|GetMovementState))
  (return (Utilities|Enum|Equal(Enum) (Utilities|Array|Get(acopy) _movementstate (Utilities|Array|LastIndex _movementstate)) "NewEnumerator0")))

(fn OnRepLootedWeapon
  (bind _lootedweapon (Variables|Default|GetLootedWeapon))
  (bind _lootedweapon_2 (Variables|Default|GetLootedWeapon))
  (bind _weapon (Variables|/Game/Blueprints/Weapons/BP_WeaponBase.BP_WeaponBase_C|GetWeapon _lootedweapon))
  (Physics|SetSimulatePhysics _weapon false)
  (Collision|SetCollisionEnabled _weapon "NoCollision") ; 取得している時の衝突削除
  (Collision|SetCollisionEnabled (Variables|/Game/Blueprints/Weapons/BP_WeaponBase.BP_WeaponBase_C|GetCollisionSphere (Variables|Default|GetLootedWeapon)) "NoCollision") ; 所持武器を取得されないように設定
  (Transformation|AttachComponentToComponent (Variables|/Game/Blueprints/Weapons/BP_WeaponBase.BP_WeaponBase_C|GetWeapon _lootedweapon_2) (Variables|/Game/Blueprints/Weapons/BP_WeaponBase.BP_WeaponBase_C|GetDefaultSceneRoot _lootedweapon_2) "None" "SnapToTarget" "SnapToTarget" "SnapToTarget" true) ; 物理シミュするとDefaultSceneRootから切り離されるため再接続
  (if (Utilities|Enum|Equal(Enum) (Variables|Default|GetEquippedWeapon) "NewEnumerator0") ; 武器無しからの取得なら手に持つ
    (Transformation|AttachComponentToComponent (Variables|Default|GetLootedWeapon) (Variables|Character|GetMesh) (Utilities|Select :Index (Variables|/Game/Blueprints/Weapons/BP_WeaponBase.BP_WeaponBase_C|GetWeaponType (Variables|Default|GetLootedWeapon)) :NewEnumerator0 "None" :NewEnumerator1 "S_Pistol" :NewEnumerator2 "S_Rifle") "SnapToTarget" "SnapToTarget" "SnapToTarget" true) ; 取得したらメッシュにアタッチ
    (else
      (Transformation|AttachComponentToComponent (Variables|Default|GetLootedWeapon) (Variables|Character|GetMesh) (Utilities|Select :Index (Variables|/Game/Blueprints/Weapons/BP_WeaponBase.BP_WeaponBase_C|GetWeaponType (Variables|Default|GetLootedWeapon)) :NewEnumerator0 "None" :NewEnumerator1 "S_Weapon_Thigh" :NewEnumerator2 "S_Weapon_Back") "SnapToTarget" "SnapToTarget" "SnapToTarget" true) ; 取得したらメッシュにアタッチ
    )))

(fn GetPlayerRef
  (return self) ; PlayerはBP_PlayerBaseである
)